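; GunPickup is a pickup actor that arms the player and triggers a zombie encounter when overlapped.
; On overlap with RR_PlayerPawn, it turns on the pawn's point light and sets its Gun flag.
; It then disables the gate on the referenced ZombieBars, calls LightsOffOn on the Lights actor, spawns ZombieTest at two spawn points, and destroys itself.
; Failed casts on the bars or lights stop the remaining steps.
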(event `self.ReceiveActorBeginOverlap`
  (params (OtherActor :type "Actor Object Reference"))
  (bind _asrr_player_pawn (cast `/Game/Blueprint/RR_PlayerPawn` OtherActor))
  (`SceneComponent.SetVisibility` (`/Game/Blueprint/RR_PlayerPawn.PointLight1` _asrr_player_pawn) true false)
  (set `/Game/Blueprint/RR_PlayerPawn.Gun` true _asrr_player_pawn)
  (bind _asbars (cast `/Game/Bars` (`self.ZombieBars`)))
  (`/Game/Bars.DisableGate` _asbars)
  (bind _aslights_bp (cast `/Game/Blueprint/LightsBP` (`self.Lights`)))
  (`/Game/Blueprint/LightsBP.LightsOffOn` _aslights_bp)
  (`|SpawnActorFromClass` "/Game/Blueprint/ZombieTest.ZombieTest_C" (`self.GetTransform` (`self.ZombieSquareSpawn1`)) "Undefined" "OverrideRootScale" null null)
  (`|SpawnActorFromClass` "/Game/Blueprint/ZombieTest.ZombieTest_C" (`self.GetTransform` (`self.ZombieSquareSpawn2`)) "Undefined" "OverrideRootScale" null null)
  (`self.K2_DestroyActor`))

(fn `UserConstructionScript`)