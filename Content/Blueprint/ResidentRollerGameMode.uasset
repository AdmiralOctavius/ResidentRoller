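; Game mode for Resident Roller that owns the level HUD and keeps its ammo readout current.
; On BeginPlay it creates the LevelUI widget, plays the This_House sound in 2D and seeds the ammo count from the player pawn.
; ChangeAmmo stores a new count, prints a debug message and writes the value straight into the widget's ammo text.
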(event `self.ReceiveBeginPlay`
  (bind _returnvalue (`|CreateWidget` "/Game/Widgets/LevelUI.LevelUI_C"))
  (set `self.WidgetHandle` _returnvalue)
  (`UserWidget.AddToViewport` _returnvalue 0)
  (`GameplayStatics.PlaySound2D` "/Game/Audio/This_House.This_House" 0.75 1.0 0.0 null null)
  (bind _asrr_player_pawn (cast `/Game/Blueprint/RR_PlayerPawn` (`GameplayStatics.GetPlayerPawn` 0)))
  (set `self.Ammo Count` (`/Game/Blueprint/RR_PlayerPawn.Ammo` _asrr_player_pawn))
  (bind _aslevel_ui (cast `/Game/Widgets/LevelUI` (`self.WidgetHandle`)))
  (`TextBlock.SetText` (`/Game/Widgets/LevelUI.AmmoCountUI` _aslevel_ui) (`KismetTextLibrary.Conv_IntToText` (`self.Ammo Count`))))

(fn `ChangeAmmo`
  (params (ammcount :type Integer :default 12))
  (`KismetSystemLibrary.PrintString` (`KismetStringLibrary.Concat_StrStr` "Game Mode Change Ammo, ammo is: " (`KismetStringLibrary.Conv_IntToString` ammcount)))
  (bind _output_get (set `self.Ammo Count` ammcount))
  (bind _aslevel_ui (cast `/Game/Widgets/LevelUI` (`self.WidgetHandle`)))
  (`TextBlock.SetText` (`/Game/Widgets/LevelUI.AmmoCountUI` _aslevel_ui) (`KismetTextLibrary.Conv_StringToText` (`KismetStringLibrary.Conv_IntToString` _output_get))))

(fn `UserConstructionScript`)