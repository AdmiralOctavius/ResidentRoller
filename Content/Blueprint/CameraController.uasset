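; Camera controller actor that switches the first player's view between two cameras, Camera1 and Camera2.
; On BeginPlay it sets the view to Camera1 and enables its own input.
; The Camera input action flips a Toggle boolean and calls SetViewTargetWithBlend on the other camera.
; A CameraSwap function duplicates the same toggle logic, but the event graph does not call it.
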(event `self.ReceiveBeginPlay`
  (`PlayerController.SetViewTargetWithBlend` (`GameplayStatics.GetPlayerController` 0) (`self.Camera1`) 0.0 "VTBlend_Linear" 0.0 false)
  (set `self.Toggle` false)
  (`self.EnableInput` (`GameplayStatics.GetPlayerController` 0)))

(event `self.ReceiveTick`
  (params (DeltaSeconds :type "Float (single-precision)")))

(event `InputAction|Camera`
  (params (Key :type "Key Structure"))
  (:`Pressed`
    (if (`self.Toggle`)
      (`PlayerController.SetViewTargetWithBlend` (`GameplayStatics.GetPlayerController` 0) (`self.Camera1`) 0.0 "VTBlend_Linear" 0.0 false)
      (set `self.Toggle` false)
      (else
        (`PlayerController.SetViewTargetWithBlend` (`GameplayStatics.GetPlayerController` 0) (`self.Camera2`) 0.0 "VTBlend_Linear" 0.0 false)
        (set `self.Toggle` true)))))

(fn `CameraSwap`
  (if (`self.Toggle`)
    (`PlayerController.SetViewTargetWithBlend` (`GameplayStatics.GetPlayerController` 0) (`self.Camera1`) 0.0 "VTBlend_Linear" 0.0 false)
    (set `self.Toggle` false)
    (else
      (`PlayerController.SetViewTargetWithBlend` (`GameplayStatics.GetPlayerController` 0) (`self.Camera2`) 0.0 "VTBlend_Linear" 0.0 false)
      (set `self.Toggle` true))))

(fn `UserConstructionScript`)