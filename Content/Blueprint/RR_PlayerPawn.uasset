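; Player pawn for Resident Roller that drives forward and back, turns by yaw input and rolls sideways through physics impulses on its cube.
; While Gun is set, firing spends ammo, updates the game mode and line-traces from FirePoint, destroying zombies or toggling target buttons.
; Holding SlowTurn lowers turn speed and shows a point light when armed.
; The trace endpoint is a flattened, scaled forward vector without the start offset.
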(event `self.ReceiveTick`
  (params (DeltaSeconds :type "Float (single-precision)"))
  (if (`self.Gun`)
    (`SceneComponent.SetVisibility` (`self.Cylinder`) true false)))

(event `InputAxis|LeftRight`
  (params (AxisValue :type "Float (single-precision)")))

(event `InputAction|Fire`
  (params (Key :type "Key Structure"))
  (bind _firepoint (`self.FirePoint`))
  (:`Pressed`
    (if (`self.Gun`)
      (if (> (`self.Ammo`) 0)
        (`/Engine/EditorBlueprintResources/StandardMacros.DecrementInt` (`self.Ammo`)
          (:`  `
            (bind _asresident_roller_game_mode (cast `/Game/Blueprint/ResidentRollerGameMode` (`GameplayStatics.GetGameMode`)))
            (`/Game/Blueprint/ResidentRollerGameMode.ChangeAmmo` _asresident_roller_game_mode (`self.Ammo`))
            (`GameplayStatics.PlaySoundAtLocation` "/Game/Audio/128296__xenonn__layered-gunshot-0.128296__xenonn__layered-gunshot-0" (`self.K2_GetActorLocation`) (struct) 0.5 1.0 0.0 null null null)
            (bind (_outhit _returnvalue) (`KismetSystemLibrary.LineTraceSingle` :`Start` (`SceneComponent.K2_GetComponentLocation` _firepoint) :`End` (* (`SceneComponent.GetForwardVector` _firepoint) (10000.0 10000.0 0.0)) :`TraceChannel` "TraceTypeQuery1" :`DrawDebugType` "ForDuration" :`DrawTime` 1.0))
            (if _returnvalue
              (bind _aszombie_test (cast `/Game/Blueprint/ZombieTest` (`.HitActor` (`GameplayStatics.BreakHitResult` _outhit)))
                (:`then`
                  (`GameplayStatics.PlaySound2D` "/Game/Audio/376818__original-sound__2-impact-wet.376818__original-sound__2-impact-wet" 3.0 1.0 0.0 null null)
                  (`self.K2_DestroyActor` _aszombie_test))
                (:`CastFailed`
                  (bind _astarget_button (cast `/Game/Blueprint/TargetButton` (`.HitActor` (`GameplayStatics.BreakHitResult` _outhit))))
                  (`/Game/Blueprint/TargetButton.LightsOnOff` _astarget_button))))))
        (else
          (`GameplayStatics.PlaySound2D` "/Game/Audio/151068__vabadus__beretta-m9-hammer-click.151068__vabadus__beretta-m9-hammer-click" 1.0 1.0 0.0 null null))))))

(event `InputAxis|ForwardBack`
  (params (AxisValue :type "Float (single-precision)"))
  (`self.AddMovementInput` (`self.GetActorForwardVector`) AxisValue))

(event `InputAction|SlowTurn`
  (params (Key :type "Key Structure"))
  (:`Pressed`
    (set `self.Turning Speed` 0.5)
    (if (`self.Gun`)
      (`SceneComponent.SetVisibility` (`self.PointLight`) true false)))
  (:`Released`
    (set `self.Turning Speed` 2.0)
    (if (`self.Gun`)
      (`SceneComponent.SetVisibility` (`self.PointLight`) false false))))

(event `InputAxis|LeftRight`
  (params (AxisValue :type "Float (single-precision)"))
  (set `self.LeftRightAxis` AxisValue)
  (`self.AddControllerYawInput` (* AxisValue (`self.Turning Speed`))))

(event `InputAction|RollRight`
  (params (Key :type "Key Structure"))
  (:`Pressed`
    (`PrimitiveComponent.AddImpulse` (`self.Cube`) (* (`SceneComponent.GetRightVector` (`self.Cube`)) (`self.VelocityPush`)) "None" false)))

(event `InputAction|RollLeft`
  (params (Key :type "Key Structure"))
  (:`Pressed`
    (`PrimitiveComponent.AddImpulse` (`self.Cube`) (* (`SceneComponent.GetRightVector` (`self.Cube`)) (* (`self.VelocityPush`) -1.0)) "None" false)))

(fn `UserConstructionScript`)