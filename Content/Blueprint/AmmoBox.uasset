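; AmmoBox is a pickup actor that gives its AmmoCount to an overlapping RR_PlayerPawn and destroys itself.
; On overlap it prints a debug message, adds the ammo to the pawn, then passes the new total to ResidentRollerGameMode's ChangeAmmo.
; The construction script creates a dynamic material on the Cube and tints BoxColor green, yellow or red by AmmoCount tier, leaving counts above the top tier untinted.
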(event `self.ReceiveActorBeginOverlap`
  (params (OtherActor :type "Actor Object Reference"))
  (`KismetSystemLibrary.PrintString` "Hello")
  (bind _asrr_player_pawn (cast `/Game/Blueprint/RR_PlayerPawn` OtherActor))
  (`self.K2_DestroyActor`)
  (bind _output_get (set `/Game/Blueprint/RR_PlayerPawn.Ammo` (+ (`/Game/Blueprint/RR_PlayerPawn.Ammo` _asrr_player_pawn) (`self.AmmoCount`)) _asrr_player_pawn))
  (bind _asresident_roller_game_mode (cast `/Game/Blueprint/ResidentRollerGameMode` (`GameplayStatics.GetGameMode`)))
  (`/Game/Blueprint/ResidentRollerGameMode.ChangeAmmo` _asresident_roller_game_mode _output_get))

(fn `UserConstructionScript`
  (bind _returnvalue (`KismetMaterialLibrary.CreateDynamicMaterialInstance` (`PrimitiveComponent.GetMaterial` (`self.Cube`) 0)))
  (`PrimitiveComponent.SetMaterial` (`self.Cube`) 0 _returnvalue)
  (if (<= (`self.AmmoCount`) 6)
    (`MaterialInstanceDynamic.SetVectorParameterValue` _returnvalue "BoxColor" (make `LinearColor` 0.0 0.229167 0.037951 1.0))
    (elif (<= (`self.AmmoCount`) 12)
      (`MaterialInstanceDynamic.SetVectorParameterValue` _returnvalue "BoxColor" (make `LinearColor` 1.0 1.0 0.0 1.0))
      (elif (<= (`self.AmmoCount`) 24)
        (`MaterialInstanceDynamic.SetVectorParameterValue` _returnvalue "BoxColor" (make `LinearColor` 1.0 0.0 0.0 1.0))))))