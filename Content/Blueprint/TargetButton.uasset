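; TargetButton is a button actor apparently meant to let a player in its trigger space switch lights, but most of its logic is disconnected.
; BeginPlay only enables input from the first player controller; the overlap and Tick events do nothing.
; Unwired nodes would track RR_PlayerPawn presence, toggle a prompt widget and call LightsOnOff.
; LightsOnOff casts the Lights reference to LightsBP and toggles its PointLight's visibility.
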(event `self.ReceiveBeginPlay`
  (`self.EnableInput` (`GameplayStatics.GetPlayerController` 0)))

(event `self.ReceiveActorBeginOverlap`
  (params (OtherActor :type "Actor Object Reference")))

(event `self.ReceiveActorEndOverlap`
  (params (OtherActor :type "Actor Object Reference")))

(event `self.ReceiveTick`
  (params (DeltaSeconds :type "Float (single-precision)")))

(event `InputAction|Interact`
  (params (Key :type "Key Structure")))

(fn `LightsOnOff`
  (bind _aslights_bp (cast `/Game/Blueprint/LightsBP` (`self.Lights`)))
  (`SceneComponent.ToggleVisibility` (`/Game/Blueprint/LightsBP.PointLight` _aslights_bp) false))

(fn `UserConstructionScript`)