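; LightsBP is a light group actor whose lights switch on and off through the LightsOffOn function.
; Each call flips the LightOn flag and sets visibility on the Scene component and all its children.
; The first call also destroys the Cube component, tracked as a one-time blocker by DestroyedBlocker.
; Construction script nodes for placing five point lights from Light variables are disconnected, and the event graph is empty.
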(fn `LightsOffOn`
  (if (not (`self.DestroyedBlocker`))
    (`ActorComponent.K2_DestroyComponent` (`self.Cube`))
    (set `self.DestroyedBlocker` true))
  (if (`self.LightOn`)
    (`SceneComponent.SetVisibility` (`self.Scene`) false true)
    (set `self.LightOn` false)
    (else
      (`SceneComponent.SetVisibility` (`self.Scene`) true true)
      (set `self.LightOn` true))))

(fn `UserConstructionScript`)