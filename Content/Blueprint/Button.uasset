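; One-shot interactable button that triggers LightsOffOn on a referenced LightsBP actor when Interact is pressed in range.
; It enables input from player controller 0 on BeginPlay and tracks range through actor overlap events.
; Widget visibility toggles as RR_PlayerPawn enters or leaves, though any overlapping actor changes the in-range flag.
; The first successful press locks the button and hides its point light.
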(event `self.ReceiveBeginPlay`
  (`self.EnableInput` (`GameplayStatics.GetPlayerController` 0)))

(event `self.ReceiveActorBeginOverlap`
  (params (OtherActor :type "Actor Object Reference"))
  (set `self.PlayerInSpace` true)
  (cast `/Game/Blueprint/RR_PlayerPawn` OtherActor)
  (`SceneComponent.ToggleVisibility` (`self.Widget`) false :!label _label))

(event `self.ReceiveActorEndOverlap`
  (params (OtherActor :type "Actor Object Reference"))
  (set `self.PlayerInSpace` false)
  (cast `/Game/Blueprint/RR_PlayerPawn` OtherActor)
  (goto _label))

(event `self.ReceiveTick`
  (params (DeltaSeconds :type "Float (single-precision)")))

(event `InputAction|Interact`
  (params (Key :type "Key Structure"))
  (:`Pressed`
    (if (`self.PlayerInSpace`)
      (if (not (`self.PressedOnce`))
        (bind _aslights_bp (cast `/Game/Blueprint/LightsBP` (`self.Lights`)))
        (`/Game/Blueprint/LightsBP.LightsOffOn` _aslights_bp)
        (set `self.PressedOnce` true)
        (`SceneComponent.SetVisibility` (`self.PointLight`) false false)))))

(fn `UserConstructionScript`)