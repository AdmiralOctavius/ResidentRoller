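; Test zombie pawn that chases the player or wanders on the navmesh, playing a looping walk animation.
; BeginPlay applies Speed to FloatingPawnMovement and starts a one-second looping timer that re-evaluates movement.
; Within WanderVar range, a complete synchronous path triggers AIMoveTo on the player; otherwise it moves to a random reachable point within that same radius.
; Manual offset and rotation steering nodes remain unwired, alongside debug prints.
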(event `self.ReceiveBeginPlay`
  (`KismetSystemLibrary.K2_SetTimerDelegate` (delegate `ZombieMove`) 1.0 true)
  (`SkeletalMeshComponent.PlayAnimation` (`self.SkeletalMesh`) "/Game/ZombieEnemyAssets/zombie-walk_Anim.zombie-walk_Anim" true)
  (bind _output_get (set `FloatingPawnMovement.MaxSpeed` (`self.Speed`) (`self.FloatingPawnMovement`)))
  (`KismetSystemLibrary.PrintString` (`KismetStringLibrary.Conv_DoubleToString` _output_get)))

(event `self.ReceiveTick`
  (params (DeltaSeconds :type "Float (single-precision)")))

(event `ZombieMove`
  (bind _returnvalue (`self.K2_GetActorLocation`))
  (bind _returnvalue_2 (`self.K2_GetActorLocation` (`GameplayStatics.GetPlayerPawn` 0)))
  (bind (_randomlocation _returnvalue_3) (`NavigationSystemV1.K2_GetRandomReachablePointInRadius` (`self.K2_GetActorLocation`) (`self.WanderVar`) null null))
  (if (<= (`KismetMathLibrary.VSizeXY` (- _returnvalue _returnvalue_2)) (`self.WanderVar`))
    (bind _returnvalue_4 (`NavigationSystemV1.FindPathToLocationSynchronously` _returnvalue _returnvalue_2 null null))
    ;[1 1 1] Validating Path
    (if (and (`NavigationPath.IsValid` _returnvalue_4) (not (`NavigationPath.IsPartial` _returnvalue_4)))
      (`|AIMoveTo` self (0.0 0.0 0.0) (`GameplayStatics.GetPlayerPawn` 0))
      (elif _returnvalue_3
        (`|AIMoveTo` self _randomlocation null :!label _label)))
    (else
      (`KismetSystemLibrary.PrintString` "Failed Distance")
      (goto _label))))

(fn `UserConstructionScript`)